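; Example modular cowboy character that re-randomizes its look every second after BeginPlay, showcasing the character kit's variations.
; The construction script slaves each body-part mesh to the main Mesh via master pose and sets that Mesh's Visibility material parameter to zero.
; A self-calling ReSetup event picks random part meshes, swaps materials by slot name with shared skin and hair colors, and toggles accessory visibility.
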(event `self.ReceiveBeginPlay`
  ;[1 1 1] Begin Play
  (`KismetSystemLibrary.Delay` 1.0)
  (`self.Re Setup`))

(event `Re Setup`
  (bind _beardsm (`self.BeardSM`))
  (bind _torsosm (`self.TorsoSM`))
  (bind _pantssm (`self.PantsSM`))
  (bind _hairsm (`self.HairSM`))
  (bind _glassessm (`self.GlassesSM`))
  (bind _holstersm (`self.HolsterSM`))
  (bind _returnvalue (select `bool` (`self.SkinColor`) :`false` "/Game/ModularCowboyCharacter/Materials/M_CS_Skin_W.M_CS_Skin_W" :`true` "/Game/ModularCowboyCharacter/Materials/M_CS_Skin_B.M_CS_Skin_B" :!type "MaterialInterface Object Reference"))
  ;[1 1 1] Loop Begin
  ;[1 1 1] Random Cloth
  (`SkinnedMeshComponent.SetSkinnedAssetAndUpdate` (`self.Torso`) (`|GetArrayItem` _torsosm (- (`KismetMathLibrary.RandomIntegerInRange` 1 (`KismetArrayLibrary.Array_Length` _torsosm)) 1)) true)
  (`SkinnedMeshComponent.SetSkinnedAssetAndUpdate` (`self.Pants`) (`|GetArrayItem` _pantssm (- (`KismetMathLibrary.RandomIntegerInRange` 1 (`KismetArrayLibrary.Array_Length` _pantssm)) 1)) true)
  (`SkinnedMeshComponent.SetSkinnedAssetAndUpdate` (`self.Hair`) (`|GetArrayItem` _hairsm (- (`KismetMathLibrary.RandomIntegerInRange` 1 (`KismetArrayLibrary.Array_Length` _hairsm)) 1)) true)
  (`SkinnedMeshComponent.SetSkinnedAssetAndUpdate` (`self.Glasses`) (`|GetArrayItem` _glassessm (- (`KismetMathLibrary.RandomIntegerInRange` 1 (`KismetArrayLibrary.Array_Length` _glassessm)) 1)) true)
  (`SkinnedMeshComponent.SetSkinnedAssetAndUpdate` (`self.Holster`) (`|GetArrayItem` _holstersm (- (`KismetMathLibrary.RandomIntegerInRange` 1 (`KismetArrayLibrary.Array_Length` _holstersm)) 1)) true)
  (`SkinnedMeshComponent.SetSkinnedAssetAndUpdate` (`self.Beard`) (`|GetArrayItem` _beardsm (- (`KismetMathLibrary.RandomIntegerInRange` 1 (`KismetArrayLibrary.Array_Length` _beardsm)) 1)) true)
  ;[1 1 1] Simple Random Color Setup
  (set `self.SkinColor` (`KismetMathLibrary.RandomBool`))
  (set `self.HairColor` (`KismetMathLibrary.RandomIntegerInRange` 0 3))
  (for _array_element (`|MakeArray` (`self.Head`) (`self.Pants`) (`self.Shoes`) (`self.Hair`) (`self.Glasses`) (`self.Beard`) (`self.Holster`) (`self.Torso`))
    (`PrimitiveComponent.SetMaterialByName` _array_element "Mat1" (select `int` (`KismetMathLibrary.RandomIntegerInRange` 0 1) :`0` "/Game/ModularCowboyCharacter/Materials/M_CS_Black.M_CS_Black" :`1` "/Game/ModularCowboyCharacter/Materials/M_CS_Brown.M_CS_Brown" :!type "MaterialInterface Object Reference"))
    (`PrimitiveComponent.SetMaterialByName` _array_element "Mat2" (select `int` (`KismetMathLibrary.RandomIntegerInRange` 0 3) :`0` "/Game/ModularCowboyCharacter/Materials/M_CS_Black.M_CS_Black" :`1` "/Game/ModularCowboyCharacter/Materials/M_CS_Blue.M_CS_Blue" :`2` "/Game/ModularCowboyCharacter/Materials/M_CS_Red.M_CS_Red" :`3` "/Game/ModularCowboyCharacter/Materials/M_CS_White.M_CS_White" :!type "MaterialInterface Object Reference"))
    (`PrimitiveComponent.SetMaterialByName` _array_element "Pants" (select `int` (`KismetMathLibrary.RandomIntegerInRange` 0 1) :`0` "/Game/ModularCowboyCharacter/Materials/M_CS_Black.M_CS_Black" :`1` "/Game/ModularCowboyCharacter/Materials/M_CS_Blue.M_CS_Blue" :!type "MaterialInterface Object Reference"))
    (`PrimitiveComponent.SetMaterialByName` _array_element "Shoes" (select `int` (`KismetMathLibrary.RandomIntegerInRange` 0 2) :`0` "/Game/ModularCowboyCharacter/Materials/M_CS_Black.M_CS_Black" :`1` "/Game/ModularCowboyCharacter/Materials/M_CS_Brown.M_CS_Brown" :`2` "/Game/ModularCowboyCharacter/Materials/M_CS_White.M_CS_White" :!type "MaterialInterface Object Reference"))
    (`PrimitiveComponent.SetMaterialByName` _array_element "Hair" (select `int` (`self.HairColor`) :`0` "/Game/ModularCowboyCharacter/Materials/M_CS_Black.M_CS_Black" :`1` "/Game/ModularCowboyCharacter/Materials/M_CS_Brown.M_CS_Brown" :`2` "/Game/ModularCowboyCharacter/Materials/M_CS_Yellow.M_CS_Yellow" :`3` "/Game/ModularCowboyCharacter/Materials/M_CS_Red.M_CS_Red" :!type "MaterialInterface Object Reference"))
    (`PrimitiveComponent.SetMaterialByName` _array_element "Skin" _returnvalue)
    (`PrimitiveComponent.SetMaterialByName` _array_element "Skin2" _returnvalue)
    (`PrimitiveComponent.SetMaterialByName` _array_element "Flesh" _returnvalue))
  ;[1 1 1] Random Accessoire Visibility
  (for _array_element_2 (`|MakeArray` (`self.Beard`) (`self.Glasses`) (`self.Holster`))
    (`SceneComponent.SetVisibility` _array_element_2 (`KismetMathLibrary.RandomBool`) false))
  (`SceneComponent.SetVisibility` (`self.Hat`) (`KismetMathLibrary.RandomBool`) false)
  ;[1 1 1] LoopEnd
  (`KismetSystemLibrary.Delay` 1.0)
  (`self.Re Setup`))

(fn `UserConstructionScript`
  ;[1 1 1] Set Master Bone Component
  (`SkinnedMeshComponent.SetLeaderPoseComponent` (`self.Pants`) (`self.Mesh`) false)
  (`SkinnedMeshComponent.SetLeaderPoseComponent` (`self.Shoes`) (`self.Mesh`) false)
  (`SkinnedMeshComponent.SetLeaderPoseComponent` (`self.Hair`) (`self.Mesh`) false)
  (`SkinnedMeshComponent.SetLeaderPoseComponent` (`self.Glasses`) (`self.Mesh`) false)
  (`SkinnedMeshComponent.SetLeaderPoseComponent` (`self.Holster`) (`self.Mesh`) false)
  (`SkinnedMeshComponent.SetLeaderPoseComponent` (`self.Beard`) (`self.Mesh`) false)
  (`SkinnedMeshComponent.SetLeaderPoseComponent` (`self.Head`) (`self.Mesh`) false)
  (`SkinnedMeshComponent.SetLeaderPoseComponent` (`self.Torso`) (`self.Mesh`) false)
  (`MeshComponent.SetScalarParameterValueOnMaterials` (`self.Mesh`) "Visibility" 0.0))
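; BP_BillController is a player controller that makes the BP_Bill character in the level track the mouse cursor.
; On BeginPlay it adds the IMC_Player Enhanced Input mapping context, caches the first BP_Bill found in the level and shows the cursor.
; Every Tick it traces under the cursor on the Visibility channel and passes the hit location to Bill through LookAtMessage.
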(event `self.ReceiveBeginPlay`
  (`|ExecutionSequence`
    (:`then_0`
      ;[1 1 1] 绑定IMC
      (`EnhancedInputSubsystemInterface.AddMappingContext` (pcsubsystem `EnhancedInputLocalPlayerSubsystem` (`GameplayStatics.GetPlayerController` 0)) "/Game/JialeChen/Input/IMC_Player.IMC_Player" 0 (struct)))
    (:`then_1`
      ;[1 1 1] 获取场景中BP_Bill的实例——Bill
      (bind _outactors (`GameplayStatics.GetAllActorsOfClass` "/Game/JialeChen/BP/Bill/BP_Bill.BP_Bill_C"))
      (set `self.Bill` (`|GetArrayItem` _outactors)))
    (:`then_2`
      (set `self.bShowMouseCursor` true))))

(event `self.ReceiveTick`
  (params (DeltaSeconds :type "Float (single-precision)"))
  ;[1 1 1] 给Bill传入鼠标的位置
  (message `/Game/JialeChen/BP/BPI/BPI_Character.LookAt` (`self.Bill`) (`.Location` (`GameplayStatics.BreakHitResult` (`self.GetHitResultUnderCursorByChannel` "TraceTypeQuery1")))))

(fn `UserConstructionScript`)
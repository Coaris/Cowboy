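; BP_Bill is a player character that moves relative to a fixed level camera and turns to face the mouse target.
; BeginPlay caches the "StartCamera" actor and ABP_Bill, and Enhanced Input moves Bill along that camera's flattened axes.
; Lookat maps target distance between FocusMin and FocusMax to shoulder yaw, swinging both arms from straight ahead (near) to spread sideways (far).
; The resulting hand positions feed the AnimBP's AimLeft and AimRight.
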(event `self.ReceiveBeginPlay`
  ;[1 1 1] 获得关卡相机的引用
  (bind _outactors (`GameplayStatics.GetAllActorsOfClass` "/Script/Engine.CameraActor"))
  (for _array_element _outactors
    (if (`KismetStringLibrary.EqualEqual_StrStr` (`KismetSystemLibrary.GetDisplayName` _array_element) "StartCamera")
      (set `self.MainCamera` _array_element)
      ;[1 1 1] Get this Bill's Animation Class
      (bind _asabp_bill (cast `/Game/JialeChen/Animations/Bill/ABP_Bill` (`SkeletalMeshComponent.GetAnimInstance` (`self.Mesh`))))
      (set `self.animClass` _asabp_bill))))

(event `EnhancedInput|/Game/JialeChen/Input/IA_Move`
  (params (ActionValue :type "Vector2D Structure") (ElapsedSeconds :type "Float (double-precision)") (TriggeredSeconds :type "Float (double-precision)") (InputAction :type "InputAction Object Reference" :default "/Game/JialeChen/Input/IA_Move.IA_Move"))
  (bind (_returnvalue_x _returnvalue_y) (`KismetMathLibrary.BreakVector2D` (`KismetMathLibrary.Normal2D` ActionValue)))
  (bind _maincamera (`self.MainCamera`))
  (bind (_returnvalue_x_2 _returnvalue_y_2) (`KismetMathLibrary.BreakVector` (`self.GetActorForwardVector` _maincamera)))
  ;[1 1 1] 使用EIS移动
  (:`Triggered`
    (`|ExecutionSequence`
      (:`then_0`
        (`self.AddMovementInput` (`self.GetActorRightVector` _maincamera) _returnvalue_x))
      (:`then_1`
        (`self.AddMovementInput` (`KismetMathLibrary.Normal` (`KismetMathLibrary.MakeVector` _returnvalue_x_2 _returnvalue_y_2)) _returnvalue_y)))))

(event `self.LookAt`
  (params (lookAtTarget :type "Vector Structure"))
  (bind (_returnvalue_x _returnvalue_y) (`KismetMathLibrary.BreakVector` (`self.K2_GetActorLocation`)))
  (bind (_returnvalue_x_2 _returnvalue_y_2) (`KismetMathLibrary.BreakVector` (`self.K2_GetActorLocation`)))
  (bind _focusmin (`self.focusMin`))
  (bind _returnvalue (`KismetMathLibrary.Vector_Distance` (`KismetMathLibrary.MakeVector` lookAtTarget_X lookAtTarget_Y) (`KismetMathLibrary.MakeVector` _returnvalue_x_2 _returnvalue_y_2)))
  ;[1 1 1] 从接口函数LookAt得到鼠标位置，看向鼠标方向
  (`self.K2_SetActorRotation` (`KismetMathLibrary.FindLookAtRotation` (`KismetMathLibrary.MakeVector` _returnvalue_x _returnvalue_y) (`KismetMathLibrary.MakeVector` lookAtTarget_X lookAtTarget_Y)))
  ;[1 1 1] Aim
  ;;[1 1 1] 当鼠标距离比小焦距小时
  (if (<= _returnvalue (`self.focusMin`))
    ;;[1 1 1] 向前伸直双臂
    (`|ExecutionSequence`
      (:`then_0`
        (`SceneComponent.K2_SetRelativeRotation` (`self.RightShoulder`) (`KismetMathLibrary.MakeRotator` 0.0 0.0 90.0) false false)
        (`self.AimRight` (`self.animClass`) (`SceneComponent.K2_GetComponentLocation` (`self.RightHand`)) :!label _label))
      (:`then_1`
        (`SceneComponent.K2_SetRelativeRotation` (`self.LeftShoulder`) (`KismetMathLibrary.MakeRotator` 0.0 0.0 90.0) false false)
        (`self.AimLeft` (`self.animClass`) (`SceneComponent.K2_GetComponentLocation` (`self.LeftHand`)) :!label _label_2)))
    (else
      ;;[1 1 1] 当鼠标距离比大焦距大时
      (if (>= _returnvalue (`self.focusMax`))
        ;;[1 1 1] 两侧展开双臂
        (`|ExecutionSequence`
          (:`then_0`
            (`SceneComponent.K2_SetRelativeRotation` (`self.RightShoulder`) (`KismetMathLibrary.MakeRotator` 0.0 0.0 180.0) false false)
            (goto _label))
          (:`then_1`
            (`SceneComponent.K2_SetRelativeRotation` (`self.LeftShoulder`) (`KismetMathLibrary.MakeRotator` 0.0 0.0 0.0) false false)
            (goto _label_2)))
        (elif true
          ;;[1 1 1] 夹角双臂
          (set `self.aimAlpha` (/ (- _returnvalue _focusmin) (- (`self.focusMax`) _focusmin)))
          (`|ExecutionSequence`
            (:`then_0`
              (`SceneComponent.K2_SetRelativeRotation` (`self.RightShoulder`) (`KismetMathLibrary.MakeRotator` 0.0 0.0 (+ 90.0 (* (`self.aimAlpha`) 90.0))) false false)
              (goto _label))
            (:`then_1`
              (`SceneComponent.K2_SetRelativeRotation` (`self.LeftShoulder`) (`KismetMathLibrary.MakeRotator` 0.0 0.0 (- 90.0 (* (`self.aimAlpha`) 90.0))) false false)
              (goto _label_2))))))))

(fn `UserConstructionScript`)